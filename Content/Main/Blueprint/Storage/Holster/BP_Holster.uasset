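; BP_Holster is a single-item holster slot that holds grabbable actors dropped inside its overlap sphere.
; While overlapping, GrabComponents flagged IsHolster have their grab and drop events bound.
; Dropping captures the actor if the slot is empty, disabling physics and attaching it; grabbing or leaving releases it, with a resources message sent on both transitions.
; A second sphere enlarges on any overlap and resets on drop or exit.
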(event OnComponentBeginOverlap(Sphere1)
  (params (OverlappedComponent :type Primitive%20Component%20Object%20Reference) (OtherActor :type Actor%20Object%20Reference) (OtherComp :type Primitive%20Component%20Object%20Reference) (OtherBodyIndex :type Integer) (bFromSweep :type Boolean) (SweepResult :type Hit%20Result%20Structure%20%28by%20ref%29))
  ;[0.02604 0.02604 0.02604] Slot Manager and Holster
  (for _array_element (Actor|GetComponentsByClass OtherActor "/Game/Template/VR/VRTemplate/Blueprints/GrabComponent.GrabComponent_C")
    (if (Variables|/Game/Template/VR/VRTemplate/Blueprints/GrabComponent.GrabComponent_C|GetbIsHolster _array_element)
      (Utilities|Array|Add (Variables|Default|GetTrackedGrabComponemt) _array_element)
      (EventDispatchers|BindEventtoOnGrabbed _array_element (EventDispatchers|CreateEvent :!event Custom|OnGrabbedEvent))
      (EventDispatchers|BindEventtoOnDropped _array_element (EventDispatchers|CreateEvent :!event Custom|OnDropped))))
  (CallFunction|IncreaseCellSize))

(event OnComponentEndOverlap(Sphere1)
  (params (OverlappedComponent :type Primitive%20Component%20Object%20Reference) (OtherActor :type Actor%20Object%20Reference) (OtherComp :type Primitive%20Component%20Object%20Reference) (OtherBodyIndex :type Integer))
  ;[0.02604 0.02604 0.02604] Slot Manager and Holster
  (CallFunction|TryDropObject OtherActor)
  (for _array_element (Actor|GetComponentsByClass OtherActor "/Game/Template/VR/VRTemplate/Blueprints/GrabComponent.GrabComponent_C")
    ;;[0.03125 0.03125 0.03125] Minor Change
    (if (Variables|/Game/Template/VR/VRTemplate/Blueprints/GrabComponent.GrabComponent_C|GetbIsHolster _array_element)
      (Utilities|Array|RemoveItem (Variables|Default|GetTrackedGrabComponemt) _array_element)
      (EventDispatchers|UnbindEventfromOnGrabbed _array_element (EventDispatchers|CreateEvent :!event Custom|OnGrabbedEvent))
      (EventDispatchers|UnbindEventfromOnDropped _array_element (EventDispatchers|CreateEvent :!event Custom|OnDropped))))
  (CallFunction|DecreaseCellSize))

(event Custom|OnGrabbedEvent
  (params (Motion%20Controller :type Motion%20Controller%20Component%20Object%20Reference) (BoneName :type Name) (HandMesh :type Skeletal%20Mesh%20Component%20Object%20Reference) (PhysicsHandle :type Physics%20Handle%20Component%20Object%20Reference) (hand :type E_VRHand%20Enum :default "NewEnumerator0") (Self%20References :type Grab%20Component%20Object%20Reference))
  ;[0.02604 0.02604 0.02604] Slot Manager and Holster
  (CallFunction|TryDropObject (Components|GetOwner Self%20References)))

(event Custom|OnDropped
  (params (Self%20References :type Grab%20Component%20Object%20Reference))
  ;[0.02604 0.02604 0.02604] Slot Manager and Holster
  (CallFunction|TryCaptureObject Self%20References)
  (CallFunction|DecreaseCellSize))

(event EventBeginPlay
  (Variables|Default|SetInitialSelfScale (Transformation|GetWorldScale (Variables|Default|GetSphere))))

(fn ConstructionScript)

(fn TryDropObject
  (params (Actor :type Actor%20Object%20Reference))
  (Utilities|IsValid (Variables|Default|GetHeldActor)
    (:Is%20Valid
      (if (== Actor (Variables|Default|GetHeldActor))
        (if (== (Actor|GetAttachParentActor (Variables|Default|GetHeldActor)) self)
          (Transformation|DetachFromActor (Variables|Default|GetHeldActor) "KeepWorld" "KeepWorld" "KeepWorld"))
        (Class|BPIActor|FActorResources(Message) (Variables|Default|GetHeldActor) true)
        (Variables|Default|SetHeldActor 0)))))

(fn TryCaptureObject
  (params (GrabComponent :type Grab%20Component%20Object%20Reference))
  ;[1 1 1] This Function is not call still so may not issue with thuis
  (Utilities|IsValid (Variables|Default|GetHeldActor)
    (:Is%20Not%20Valid
      (bind _output_get (Variables|Default|SetHeldActor (Components|GetOwner GrabComponent)))
      (Default|SetPrimitiveCompPhysics GrabComponent false)
      (Transformation|AttachComponentToComponent _output_get (Variables|Default|GetDefaultSceneRoot) "None" "SnapToTarget" "KeepWorld" "KeepWorld" true)
      (Class|BPIActor|FActorResources(Message) (Variables|Default|GetHeldActor) false))))

(fn IncreaseCellSize
  (Transformation|SetWorldScale3D (Variables|Default|GetSphere) (* (Variables|Default|GetInitialSelfScale) 1.5)))

(fn DecreaseCellSize
  (Transformation|SetWorldScale3D (Variables|Default|GetSphere) (Variables|Default|GetInitialSelfScale)))