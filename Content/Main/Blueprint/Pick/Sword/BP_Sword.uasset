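; BP_Sword is a grabbable sword that damages objects it strikes.
; GrabComponent events switch off mesh physics and apply a grip pose (identical for either hand) on grab, then restore physics on drop.
; A Box overlap triggers a sphere trace along the Arrow's forward vector, applying damage to the hit actor.
; FActorResources toggles the actor between its default scale and one-eighth size according to its active flag.
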(event OnGrabbed(GrabComponent)
  (params (Motion%20Controller :type Motion%20Controller%20Component%20Object%20Reference) (BoneName :type Name :default "None") (HandMesh :type Skeletal%20Mesh%20Component%20Object%20Reference) (PhysicsHandle :type Physics%20Handle%20Component%20Object%20Reference) (hand :type E_VRHand%20Enum :default "NewEnumerator0") (Self%20References :type Grab%20Component%20Object%20Reference))
  (bind _staticmesh (Variables|Default|GetStaticMesh))
  (Physics|SetSimulatePhysics (Variables|Default|GetStaticMesh) false)
  (switch Utilities|FlowControl|Switch|SwitchonE_VRHand hand
    (:NewEnumerator1
      (Transformation|SetRelativeLocationAndRotation _staticmesh "0.000000,0.500000,-2.500000" "20.000000,90.000000,-80.000000" false false))
    (:NewEnumerator2
      (Transformation|SetRelativeLocationAndRotation _staticmesh "0.000000,0.500000,-2.500000" "20.000000,90.000000,-80.000000" false false))))

(event OnDropped(GrabComponent)
  (params (Self%20References :type Grab%20Component%20Object%20Reference))
  (Physics|SetSimulatePhysics (Variables|Default|GetStaticMesh) true))

(event OnComponentBeginOverlap(Box)
  (params (OverlappedComponent :type Primitive%20Component%20Object%20Reference) (OtherActor :type Actor%20Object%20Reference) (OtherComp :type Primitive%20Component%20Object%20Reference) (OtherBodyIndex :type Integer) (bFromSweep :type Boolean) (SweepResult :type Hit%20Result%20Structure%20%28by%20ref%29))
  (bind _arrow (Variables|Default|GetArrow))
  (bind _returnvalue (Transformation|GetWorldLocation _arrow))
  (bind (_outhit _returnvalue_2) (Collision|SphereTraceForObjects _returnvalue (+ _returnvalue (* (Math|Vector|GetForwardVector _arrow) (Variables|Scaling|GetSphereTraceRadius))) 2e+01 (Utilities|Array|MakeArray "ObjectTypeQuery7") false (Utilities|Array|MakeArray self) "None"))
  (if _returnvalue_2
    (Game|Damage|ApplyDamage (.HitActor (Collision|BreakHitResult _outhit)) 1e+01 0 0)))

(event EventBeginPlay
  (bind _output_get (Variables|Scaling|SetDefaultScale (Transformation|GetActorScale3D)))
  (Variables|Scaling|SetMicroScale (/ _output_get 8.0)))

(event EventFActorResources
  (params (isActive :type Boolean))
  (if isActive
    (Transformation|SetActorScale3D (Variables|Scaling|GetDefaultScale))
    (else
      (Transformation|SetActorScale3D (Variables|Scaling|GetMicroScale)))))

(fn ConstructionScript)