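; Arrow projectile actor for the bow, launched at a variable speed and damaging what it hits.
; ArrowSpeed scales the passed value into the projectile movement's initial and max speed, then sets velocity along local forward.
; When the collision component begins overlapping, a short forward sphere trace for one object type picks the actor that takes fixed damage.
; The arrow destroys itself shortly after its projectile movement stops.
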(event OnProjectileStop(ProjectileMovement)
  (params (ImpactResult :type Hit%20Result%20Structure%20%28by%20ref%29))
  ;[1 1 1] Arrow
  (Utilities|FlowControl|Delay 2.0)
  (Actor|DestroyActor))

(event OnComponentBeginOverlap(Collision-Arrow)
  (params (OverlappedComponent :type Primitive%20Component%20Object%20Reference) (OtherActor :type Actor%20Object%20Reference) (OtherComp :type Primitive%20Component%20Object%20Reference) (OtherBodyIndex :type Integer) (bFromSweep :type Boolean) (SweepResult :type Hit%20Result%20Structure%20%28by%20ref%29))
  (bind _returnvalue (Transformation|GetActorLocation))
  ;[1 1 1] Arrow
  (bind (_outhit _returnvalue_2) (Collision|SphereTraceForObjects _returnvalue (+ _returnvalue (* (Transformation|GetActorForwardVector) 1e+02)) 2e+01 (Utilities|Array|MakeArray "ObjectTypeQuery7") false 0 "None"))
  (if _returnvalue_2
    (Game|Damage|ApplyDamage (.HitActor (Collision|BreakHitResult _outhit)) 1e+01 0 0)))

(event Custom|ArrowSpeed
  (params (Speed :type Float%20%28double-precision%29))
  (bind _returnvalue (* Speed 2e+03))
  (bind _projectilemovement (Variables|Default|GetProjectileMovement))
  ;[1 1 1] Arrow
  (Variables|/Script/Engine.ProjectileMovementComponent|SetMaxSpeed _projectilemovement _returnvalue)
  (bind _output_get (Variables|/Script/Engine.ProjectileMovementComponent|SetInitialSpeed _projectilemovement _returnvalue))
  (Game|Components|ProjectileMovement|SetVelocityinLocalSpace _projectilemovement (Math|Vector|MakeVector _output_get 0.0 0.0)))

(fn ConstructionScript)