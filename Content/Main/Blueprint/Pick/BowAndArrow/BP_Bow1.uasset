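; BP_Bow1 is a motion-controller bow that fires arrows when the grabbed string is released.
; While the bow is held, grabbing the string shows a preview arrow and starts a looping timer, apparently driving RelativePosition.
; RelativePosition clamps the string box between spline endpoints and normalizes PullBack, which sets the spawned BP_Arrow's speed on release.
; FActorResources toggles string grabbing, animation and collision, shrinking the bow when inactive.
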(event OnGrabbed(GrabBow)
  (params (Motion%20Controller :type Motion%20Controller%20Component%20Object%20Reference) (BoneName :type Name :default "None") (HandMesh :type Skeletal%20Mesh%20Component%20Object%20Reference) (PhysicsHandle :type Physics%20Handle%20Component%20Object%20Reference) (hand :type E_VRHand%20Enum :default "NewEnumerator0") (Self%20References :type Grab%20Component%20Object%20Reference))
  ;[0.01042 0.01042 0.01042] GrabBow
  (Physics|SetSimulatePhysics (Variables|Default|GetSkeletalMesh) false)
  (Variables|Default|SetisGrabbedBow true))

(event OnDropped(GrabBow)
  (params (Self%20References :type Grab%20Component%20Object%20Reference))
  ;[0.01042 0.01042 0.01042] GrabBow
  (Physics|SetSimulatePhysics (Variables|Default|GetSkeletalMesh) true)
  (Variables|Default|SetisGrabbedBow false))

(event OnGrabbed(GrabString)
  (params (Motion%20Controller :type Motion%20Controller%20Component%20Object%20Reference) (BoneName :type Name :default "None") (HandMesh :type Skeletal%20Mesh%20Component%20Object%20Reference) (PhysicsHandle :type Physics%20Handle%20Component%20Object%20Reference) (hand :type E_VRHand%20Enum :default "NewEnumerator0") (Self%20References :type Grab%20Component%20Object%20Reference))
  ;[0 0 0] GrabString
  (if (Variables|Default|GetisGrabbedBow)
    (Utilities|IsValid Motion%20Controller
      (:Is%20Valid
        (Variables|Default|SetMotion%20Controller Motion%20Controller)
        (Rendering|SetVisibility (Variables|Default|GetMesh%20-%20ArrowPreivew) true false)
        (bind _returnvalue (Utilities|Time|SetTimerbyEvent (EventDispatchers|CreateEvent :!event RelativePosition) 0.01 true))
        (Variables|Default|SetTimer _returnvalue)))))

(event OnDropped(GrabString)
  (params (Self%20References :type Grab%20Component%20Object%20Reference))
  (bind _arrow (Variables|Default|GetArrow))
  (bind _returnvalue (Transformation|GetWorldRotation _arrow))
  ;[0 0 0] GrabString
  (if (Variables|Default|GetisGrabbedBow)
    (Utilities|Time|ClearandInvalidateTimerbyHandle (Variables|Default|GetTimer))
    (Variables|Default|SetMotion%20Controller 0)
    (Transformation|SetRelativeLocation (Variables|Default|GetBox) (Math|Vector|MakeVector 0.0 1.7e+02 0.0) false true)
    (Rendering|SetVisibility (Variables|Default|GetMesh%20-%20ArrowPreivew) false false)
    (bind _returnvalue_2 (Game|SpawnActorfromClass "/Game/Main/Blueprint/Pick/BowAndArrow/BP_Arrow.BP_Arrow_C" (Math|Transform|MakeTransform (Transformation|GetWorldLocation _arrow) (Math|Rotator|MakeRotator (.roll _returnvalue) (.pitch _returnvalue) (.yaw _returnvalue))) "Undefined" "MultiplyWithRoot" self (Game|Player|GetPlayerPawn 0)))
    (Default|ArrowSpeed _returnvalue_2 (Variables|Default|GetPullBack))
    (Variables|Default|SetPullBack 0.0)))

(event EventBeginPlay
  ;[0.01042 0.01042 0.01042] Default
  (bind _output_get (Variables|Default|SetDefaultScale (Variables|/Script/Engine.SceneComponent|GetRelativeScale3D (Variables|Default|GetMesh%20))))
  (Variables|Default|SetMicroScale (/ _output_get (Variables|Default|GetMicroScaleThreshold))))

(event EventFActorResources
  (params (isActive :type Boolean))
  (bind _grabstring (Variables|Default|GetGrabString))
  (bind _skeletalmesh (Variables|Default|GetSkeletalMesh))
  ;[0.01562 0.01562 0.01562] Actor Behaviour
  (if isActive
    (Components|Activation|SetActive _grabstring true false)
    (Transformation|SetRelativeScale3D _skeletalmesh (Variables|Default|GetDefaultScale))
    (Variables|/Script/Engine.SkeletalMeshComponent|SetbPauseAnims _skeletalmesh false)
    (Collision|SetCollisionEnabled _skeletalmesh "QueryAndPhysics")
    (else
      (Components|Activation|Deactivate _grabstring)
      (Transformation|SetRelativeScale3D _skeletalmesh (Variables|Default|GetMicroScale))
      (Variables|/Script/Engine.SkeletalMeshComponent|SetbPauseAnims _skeletalmesh true)
      (Collision|SetCollisionEnabled _skeletalmesh "NoCollision"))))

(fn ConstructionScript)

(fn RelativePosition
  (bind _motion_controller (Variables|Default|GetMotion%20Controller))
  (bind _box (Variables|Default|GetBox))
  (bind _box_2 (Variables|Default|GetBox))
  (bind _spline (Variables|Default|GetSpline))
  (bind _returnvalue (Transformation|GetWorldTransform _box))
  (bind _returnvalue_2 (Transformation|GetWorldTransform _motion_controller))
  (bind _returnvalue_3 (Spline|GetLocationatSplinePoint _spline 1 "Local"))
  (bind _returnvalue_4 (Spline|GetLocationatSplinePoint _spline 0 "Local"))
  (bind _relativelocation (Variables|/Script/Engine.SceneComponent|GetRelativeLocation _box_2))
  (bind _returnvalue_5 (Math|Transform|MakeRelativeTransform _returnvalue_2 _returnvalue))
  (bind _returnvalue_6 (+ (.y (.location _returnvalue_5)) (.y _relativelocation)))
  (bind _returnvalue_7 (Math|Float|Clamp(Float) _returnvalue_6 (.y _returnvalue_4) (.y _returnvalue_3)))
  (Transformation|SetRelativeLocation (Variables|Default|GetBox) (Math|Vector|MakeVector 0.0 _returnvalue_7 0.0) false true)
  (Variables|Default|SetPullBack (Math|Float|NormalizetoRange _returnvalue_7 (.y _returnvalue_4) (.y _returnvalue_3))))